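; Player character Blueprint with camera-yaw-relative movement, mouse look, and networked sprinting and rolling.
; Sprint sets walk speed locally and on the server for immediate client response, with OnRep_isSprinting passing the state to the AnimInstance.
; Rolling goes through a server event to a multicast that plays the Greystone roll montage and messages the AnimInstance, with montage completion requesting the server to end the roll.
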(event Custom|Server_ToggleSprint
  (params (State :type Boolean))
  ;[1 1 1] Sprinting
  (Movement|FSprintSwitch State))

(event Custom|Server_Rolling
  (params (Rolling :type Boolean))
  (if Rolling
    (Variables|Movement|SetisRolling true)
    (CallFunction|MultiRolling "/Game/PlayerCharacter/Animation/Animations/GreystoneRoll_Montage.GreystoneRoll_Montage" true (Variables|Character|GetMesh))
    (else
      (Variables|Movement|SetisRolling false)
      (CallFunction|MultiRolling "/Game/PlayerCharacter/Animation/Animations/GreystoneRoll_Montage.GreystoneRoll_Montage" false))))

(event Custom|Multi_Rolling
  (params (Roll%20Montage :type Anim%20Montage%20Object%20Reference) (isRolling :type Boolean) (InSkeletalMeshComponent :type Skeletal%20Mesh%20Component%20Object%20Reference))
  (bind _mesh (Variables|Character|GetMesh))
  (bind _returnvalue (Components|SkeletalMesh|GetAnimInstance _mesh))
  (if isRolling
    (Class|IBPHeroAnim|RollingState(Message) _returnvalue true)
    (Animation|Montage|PlayMontage InSkeletalMeshComponent Roll%20Montage
      (:OnCompleted
        (CallFunction|ServerRolling false)))
    (else
      (Class|IBPHeroAnim|RollingState(Message) _returnvalue false))))

(event EventPossessed
  (params (NewController :type Controller%20Object%20Reference))
  ;[1 1 1] Set Can Move
  (CallFunction|UpdateMovement true))

(event Input|ActionEvents|InputActionSprint
  (params (Key :type Key%20Structure :default "None"))
  ;[1 1 1] Sprinting
  (:Pressed
    (Movement|FSprintSwitch true))
  (:Released
    (Movement|FSprintSwitch false)))

(event Input|ActionEvents|InputActionRolling
  (params (Key :type Key%20Structure :default "None"))
  (:Pressed
    (if (not (Variables|Movement|GetisRolling))
      (CallFunction|ServerRolling true))))

(event Input|AxisEvents|InputAxisTurn
  (params (AxisValue :type Float%20%28single-precision%29))
  ;[1 1 1] Mouse Movement
  (Pawn|Input|AddControllerYawInput AxisValue))

(event Input|AxisEvents|InputAxisLookUp
  (params (AxisValue :type Float%20%28single-precision%29))
  ;[1 1 1] Mouse Movement
  (Pawn|Input|AddControllerPitchInput AxisValue))

(event Input|AxisEvents|InputAxisMoveForward
  (params (AxisValue :type Float%20%28single-precision%29))
  ;[1 1 1] Basic Movement
  (Pawn|Input|AddMovementInput (Math|Vector|GetForwardVector (Math|Rotator|MakeRotator 0.0 0.0 (.Yaw (Math|Rotator|BreakRotator (Pawn|GetControlRotation :!class /Script/Engine.Pawn))))) AxisValue false))

(event Input|AxisEvents|InputAxisMoveRight
  (params (AxisValue :type Float%20%28single-precision%29))
  ;[1 1 1] Basic Movement
  (Pawn|Input|AddMovementInput (Math|Vector|GetRightVector (Math|Rotator|MakeRotator 0.0 0.0 (.Yaw (Math|Rotator|BreakRotator (Pawn|GetControlRotation :!class /Script/Engine.Pawn))))) AxisValue false))

(fn ConstructionScript
  (|CallParentFunction))

(fn FSprintSwitch
  (params (SprintState :type Boolean))
  (bind _charactermovement (Variables|Character|GetCharacterMovement))
  (bind _charactermovement_2 (Variables|Character|GetCharacterMovement))
  (LocalVariables|SetLocalSprint SprintState)
  (Networking|SwitchHasAuthority
    (:Authority
      (if (LocalVariables|GetLocalSprint)
        (Variables|/Script/Engine.CharacterMovementComponent|SetMaxWalkSpeed _charactermovement (Variables|Movement|GetsprintSpeed))
        (Variables|Movement|SetisSprinting true)
        (else
          (Variables|/Script/Engine.CharacterMovementComponent|SetMaxWalkSpeed _charactermovement (Variables|Movement|GetjogSpeed))
          (Variables|Movement|SetisSprinting false)))
      (return))
    (:Remote
      (CallFunction|ServerToggleSprint (LocalVariables|GetLocalSprint))
      (if (LocalVariables|GetLocalSprint)
        (Variables|/Script/Engine.CharacterMovementComponent|SetMaxWalkSpeed _charactermovement_2 (Variables|Movement|GetsprintSpeed))
        (else
          (Variables|/Script/Engine.CharacterMovementComponent|SetMaxWalkSpeed _charactermovement_2 (Variables|Movement|GetjogSpeed))))
      (return))))

(fn OnRepIsSprinting
  (bind _mesh (Variables|Character|GetMesh))
  (bind _returnvalue (Components|SkeletalMesh|GetAnimInstance _mesh))
  (if (Variables|Movement|GetisSprinting)
    (Class|IBPHeroAnim|SprintState(Message) _returnvalue true)
    (else
      (Class|IBPHeroAnim|SprintState(Message) _returnvalue false))))